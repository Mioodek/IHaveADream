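; BP_Magnetofon is a tape recorder pickup that the first-person character collects with the interact button.
; Entering its Box casts and stores the character, sets an outline overlay material on the Cube and enables Tick, which is off by default.
; Tick polls the character's interact flag, then destroys the actor and adds the MagnetofidPickedUp widget to the viewport.
; Leaving the Box with the Player tag restores the base overlay and disables Tick.
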(event `self.ReceiveTick`
  (params (DeltaSeconds :type "Float (single-precision)"))
  (if (`/Game/IHaveADream/Player/BP_FirstPersonCharacter1.InteractButtonIsBeingPressed` (`self.As BP First Person Character`))
    (`self.K2_DestroyActor`)
    (bind _returnvalue (`|CreateWidget` "/Game/IHaveADream/Menu/UI/MagnetofidPickedUp.MagnetofidPickedUp_C"))
    (`UserWidget.AddToViewport` _returnvalue 0)))

(event `self.ReceiveBeginPlay`
  (`self.SetActorTickEnabled` false))

(event `self.Box.OnComponentBeginOverlap`
  (params (OverlappedComponent :type "PrimitiveComponent Object Reference") (OtherActor :type "Actor Object Reference") (OtherComp :type "PrimitiveComponent Object Reference") (OtherBodyIndex :type Integer) (bFromSweep :type Boolean) (SweepResult :type "HitResult Structure (by ref)"))
  (bind _asbp_first_person_character_1 (cast `/Game/IHaveADream/Player/BP_FirstPersonCharacter1` OtherActor))
  (set `self.As BP First Person Character` _asbp_first_person_character_1)
  (`MeshComponent.SetOverlayMaterial` (`self.Cube`) "/Game/IHaveADream/Menu/OutlineMaterial.OutlineMaterial")
  (`self.SetActorTickEnabled` true))

(event `self.Box.OnComponentEndOverlap`
  (params (OverlappedComponent :type "PrimitiveComponent Object Reference") (OtherActor :type "Actor Object Reference") (OtherComp :type "PrimitiveComponent Object Reference") (OtherBodyIndex :type Integer))
  (if (`self.ActorHasTag` OtherActor "Player")
    (`MeshComponent.SetOverlayMaterial` (`self.Cube`) "/Game/FPWeapon/Materials/BaseMaterial.BaseMaterial")
    (`self.SetActorTickEnabled` false)))

(fn `UserConstructionScript`)