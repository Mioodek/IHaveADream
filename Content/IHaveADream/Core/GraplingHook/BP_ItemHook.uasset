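; BP_ItemHook is a grappling hook projectile that latches onto items tagged ItemHook.
; On spawn it passes itself to the instigating player through CallStartGrappleItem.
; On hitting a tagged actor it stores it as ItemToPull, stops its movement, attaches to it and calls start grapple again.
; Any other hit tells the player to stop the grapple; the pull itself is not implemented here.
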(event `self.ReceiveBeginPlay`
  (`/Game/IHaveADream/Player/BP_FirstPersonCharacter1.StartGrappleItem` (`self.InstigatorPlayer`) self))

(event `self.CollisionComponent.OnComponentHit`
  (params (HitComponent :type "PrimitiveComponent Object Reference") (OtherActor :type "Actor Object Reference") (OtherComp :type "PrimitiveComponent Object Reference") (NormalImpulse :type "Vector Structure") (Hit :type "HitResult Structure (by ref)"))
  (if (`self.ActorHasTag` OtherActor "ItemHook")
    (bind _output_get (set `self.ItemToPull` OtherActor))
    (`MovementComponent.StopMovementImmediately` (`self.ProjectileMovement`))
    (`self.K2_AttachToActor` self _output_get "None" "KeepWorld" "KeepWorld" "KeepWorld" true)
    (`/Game/IHaveADream/Player/BP_FirstPersonCharacter1.StartGrappleItem` (`self.InstigatorPlayer`) null)
    (else
      (`/Game/IHaveADream/Player/BP_FirstPersonCharacter1.StopGrappleItem` (`self.InstigatorPlayer`)))))

(fn `UserConstructionScript`
  (`parent.UserConstructionScript`))