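; Player character component that runs a dual grappling hook: one pulls the player to walls, the other pulls items toward the player.
; Input spawns hook projectiles on press and requests a stop on release.
; Character dispatchers advance each grapple's enum state, attach or hide its cable, and destroy hooks on stop.
; While pulling, Tick drains energy and applies force to the player, in Flying mode, or to the hooked item.
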(event `self.ReceiveBeginPlay`
  (bind _playercharacter (`self.PlayerCharacter`))
  (bind _asbp_first_person_character_1 (cast `/Game/IHaveADream/Player/BP_FirstPersonCharacter1` (`self.GetOwner`)))
  (set `self.PlayerCharacter` _asbp_first_person_character_1)
  (`|ExecutionSequence`
    (:`then_0`
      (bind _asplayer_controller (cast `PlayerController` (`Pawn.GetController` (`self.PlayerCharacter`))))
      (bind _returnvalue (pcsubsystem `EnhancedInputLocalPlayerSubsystem` _asplayer_controller))
      (`/Engine/EditorBlueprintResources/StandardMacros.IsValid` _returnvalue
        (:`Is Valid`
          (`EnhancedInputSubsystemInterface.AddMappingContext` _returnvalue "/Game/IHaveADream/Player/Input/IMC_GrapplingShoots.IMC_GrapplingShoots" 0 (struct)))))
    (:`then_1`
      ; Event WallHook
      (add `/Game/IHaveADream/Player/BP_FirstPersonCharacter1.StartGrappleToWall` _playercharacter (`|CreateDelegate` :!event `StartGrappleToWall_Event`))
      (add `/Game/IHaveADream/Player/BP_FirstPersonCharacter1.StartGrapplePullToWall` _playercharacter (`|CreateDelegate` :!event `StartGrapplePullToWall_Event`))
      (add `/Game/IHaveADream/Player/BP_FirstPersonCharacter1.StopGrappleToWall` _playercharacter (`|CreateDelegate` :!event `StopGrappleToWall_Event`))
      ; Event ItemHook
      (add `/Game/IHaveADream/Player/BP_FirstPersonCharacter1.StartGrappleItem` _playercharacter (`|CreateDelegate` :!event `StartGrappleItem_Event`))
      (add `/Game/IHaveADream/Player/BP_FirstPersonCharacter1.StartGrapplePullItem` _playercharacter (`|CreateDelegate` :!event `StartGrapplePullItem_Event`))
      (add `/Game/IHaveADream/Player/BP_FirstPersonCharacter1.StopGrappleItem` _playercharacter (`|CreateDelegate` :!event `StopGrappleItem_Event`)))))

(event `StartGrappleToWall_Event`
  (params (WallHook :type "/Game/IHaveADream/Core/GraplingHook/BP_WallHook Object Reference"))
  ; Event WallHook
  (if (`|EnumEquality` (`self.GrappleWall`) "NewEnumerator1")
    (bind _output_get (set `self.Wall Hook` WallHook))
    (set `self.GrappleWall` "NewEnumerator2")
    (`CableComponent.SetAttachEndTo` (`/Game/IHaveADream/Player/BP_FirstPersonCharacter1.CableToWall` (`self.PlayerCharacter`)) _output_get "None" "None")
    (`SceneComponent.SetVisibility` (`/Game/IHaveADream/Player/BP_FirstPersonCharacter1.CableToWall` (`self.PlayerCharacter`)) true false)))

(event `StartGrappleItem_Event`
  (params (ItemHook :type "/Game/IHaveADream/Core/GraplingHook/BP_ItemHook Object Reference"))
  ; Event ItemHook
  (if (`|EnumEquality` (`self.GrappleItem`) "NewEnumerator1")
    (bind _output_get (set `self.Item Hook` ItemHook))
    (`CableComponent.SetAttachEndTo` (`/Game/IHaveADream/Player/BP_FirstPersonCharacter1.CableToItem` (`self.PlayerCharacter`)) _output_get "None" "None")
    (`SceneComponent.SetVisibility` (`/Game/IHaveADream/Player/BP_FirstPersonCharacter1.CableToItem` (`self.PlayerCharacter`)) true false)
    (set `self.GrappleItem` "NewEnumerator2")))

(event `StartGrapplePullToWall_Event`
  ; Event WallHook
  (if (`|EnumEquality` (`self.GrappleWall`) "NewEnumerator2")
    (set `self.GrappleWall` "NewEnumerator3")
    (`CharacterMovementComponent.SetMovementMode` (`Character.CharacterMovement` (`self.PlayerCharacter`)) "MOVE_Flying" 0)))

(event `StartGrapplePullItem_Event`
  ; Event ItemHook
  (if (`|EnumEquality` (`self.GrappleItem`) "NewEnumerator2")
    (`KismetSystemLibrary.PrintString` "pull")
    (set `self.GrappleItem` "NewEnumerator3")))

(event `StopGrappleToWall_Event`
  ; Event WallHook
  (if (`|EnumEquality` (`self.GrappleWall`) "NewEnumerator3")
    (`CharacterMovementComponent.SetMovementMode` (`Character.CharacterMovement` (`self.PlayerCharacter`)) "MOVE_Falling" 0))
  (set `self.GrappleWall` "NewEnumerator1")
  (`CableComponent.SetAttachEndTo` (`/Game/IHaveADream/Player/BP_FirstPersonCharacter1.CableToWall` (`self.PlayerCharacter`)) null "None" "None")
  (`SceneComponent.SetVisibility` (`/Game/IHaveADream/Player/BP_FirstPersonCharacter1.CableToWall` (`self.PlayerCharacter`)) false false)
  (`Actor.K2_DestroyActor` (`self.Wall Hook`)))

(event `StopGrappleItem_Event`
  ; Event ItemHook
  (`CableComponent.SetAttachEndTo` (`/Game/IHaveADream/Player/BP_FirstPersonCharacter1.CableToItem` (`self.PlayerCharacter`)) null "None" "None")
  (`SceneComponent.SetVisibility` (`/Game/IHaveADream/Player/BP_FirstPersonCharacter1.CableToItem` (`self.PlayerCharacter`)) false false)
  (set `self.GrappleItem` "NewEnumerator1")
  (`Actor.K2_DestroyActor` (`self.Item Hook`)))

(event `self.ReceiveTick`
  (params (DeltaSeconds :type "Float (single-precision)"))
  (bind _returnvalue_location (`KismetMathLibrary.BreakTransform` (`Actor.GetTransform` (`self.Item Hook`))))
  (bind _returnvalue_location_2 (`KismetMathLibrary.BreakTransform` (`Actor.GetTransform` (`self.Wall Hook`))))
  (`|ExecutionSequence`
    (:`then_0`
      ; GrappleWall
      (if (`|EnumEquality` (`self.GrappleWall`) "NewEnumerator3")
        (`self.Wall Hook`
          (:`then`
            (`/Game/IHaveADream/Core/Energy/AC_EnergyBase.DrainEnergy` (`/Game/IHaveADream/Player/BP_FirstPersonCharacter1.AC_PlayerEnergy` (`self.PlayerCharacter`)) 0.5)
            (`CharacterMovementComponent.AddForce` (`Character.CharacterMovement` (`self.PlayerCharacter`)) (* (`KismetMathLibrary.Normal` (`KismetMathLibrary.GetDirectionUnitVector` (`Actor.K2_GetActorLocation` (`self.PlayerCharacter`)) _returnvalue_location_2)) (`self.WallPullForce`))))
          (:`else`))))
    (:`then_1`
      ; GrappleItem
      (if (`|EnumEquality` (`self.GrappleItem`) "NewEnumerator3")
        (`self.Item Hook`
          (:`then`
            (`/Game/IHaveADream/Core/Energy/AC_EnergyBase.DrainEnergy` (`/Game/IHaveADream/Player/BP_FirstPersonCharacter1.AC_PlayerEnergy` (`self.PlayerCharacter`)) 0.5)
            (`PrimitiveComponent.AddForce` (`Actor.GetComponentByClass` (`/Game/IHaveADream/Core/GraplingHook/BP_ItemHook.ItemToPull` (`self.Item Hook`)) "/Script/Engine.PrimitiveComponent") (* (`KismetMathLibrary.Normal` (`KismetMathLibrary.GetDirectionUnitVector` _returnvalue_location (`Actor.K2_GetActorLocation` (`self.PlayerCharacter`)))) (`self.ItemPullForce`)) "None" false))
          (:`else`))))))

(event `EnhancedInput|/Game/IHaveADream/Player/Input/Actions/IA_ShootWallHook`
  (params (ActionValue :type Boolean) (ElapsedSeconds :type "Float (double-precision)") (TriggeredSeconds :type "Float (double-precision)") (InputAction :type "InputAction Object Reference" :default "/Game/IHaveADream/Player/Input/Actions/IA_ShootWallHook.IA_ShootWallHook"))
  ; Shoot Wall Hook
  (:`Started`
    (if (`|EnumEquality` (`self.GrappleWall`) "NewEnumerator1")
      (`|SpawnActorFromClass` "/Game/IHaveADream/Core/GraplingHook/BP_WallHook.BP_WallHook_C" (`self.GetTransformForBulletSpawn`) "Undefined" "MultiplyWithRoot" null (`self.PlayerCharacter`) null)))
  (:`Completed`
    (`/Game/IHaveADream/Player/BP_FirstPersonCharacter1.StopGrappleToWall` (`self.PlayerCharacter`))))

(event `EnhancedInput|/Game/IHaveADream/Player/Input/Actions/IA_ShootItemHook`
  (params (ActionValue :type Boolean) (ElapsedSeconds :type "Float (double-precision)") (TriggeredSeconds :type "Float (double-precision)") (InputAction :type "InputAction Object Reference" :default "/Game/IHaveADream/Player/Input/Actions/IA_ShootItemHook.IA_ShootItemHook"))
  ; Comment
  (:`Started`
    (if (`|EnumEquality` (`self.GrappleItem`) "NewEnumerator1")
      (`|SpawnActorFromClass` "/Game/IHaveADream/Core/GraplingHook/BP_ItemHook.BP_ItemHook_C" (`self.GetTransformForBulletSpawn`) "Undefined" "MultiplyWithRoot" null (`self.PlayerCharacter`) null)))
  (:`Completed`
    (`/Game/IHaveADream/Player/BP_FirstPersonCharacter1.StopGrappleItem` (`self.PlayerCharacter`))))