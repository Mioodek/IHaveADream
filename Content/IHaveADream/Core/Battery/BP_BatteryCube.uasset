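; BP_BatteryCube is a battery that takes energy from the player and passes it to puzzle triggers.
; Box overlaps identify the player or puzzle trigger by actor tag, then show and attach a cable to it, clearing both on exit.
; Each tick it drains the player until full and charges the puzzle until either limit is hit, through message calls.
; An energy component stores the charge, which scales the point light's intensity.
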(event `self.ReceiveTick`
  (params (DeltaSeconds :type "Float (single-precision)"))
  (bind _energydrainfromplayer (`self.EnergyDrainFromPlayer`))
  (bind _energytosendtopuzzle (`self.EnergyToSendToPuzzle`))
  ;[1 0 0] Event Tick
  (`|ExecutionSequence`
    (:`then_0`
      ;; Player
      (if (and (`self.HasPlayer`) (!= (`/Game/IHaveADream/Core/Energy/AC_EnergyBase.EnergyProcentage` (`self.AC_EnergyBase`)) 1.0))
        (message `/Game/IHaveADream/Core/Energy/BPI_HasEnergy.DrainEnergy` (`self.Player`) _energydrainfromplayer)
        (`self.Charge` _energydrainfromplayer)))
    (:`then_1`
      ;; PuzzleTrigger
      (if (and (`self.HasPuzzleTrigger`) (> (`/Game/IHaveADream/Core/Energy/AC_EnergyBase.EnergyProcentage` (`self.AC_EnergyBase`)) 0.0))
        (if (< (`/Game/IHaveADream/Core/Energy/AC_EnergyBase.EnergyProcentage` (`self.PuzzleEnergyComponent`)) 1.0)
          (message `/Game/IHaveADream/Core/Energy/BPI_HasEnergy.ChargeEnergy` (`self.Puzzle`) _energytosendtopuzzle)
          (`self.Drain` _energytosendtopuzzle))))))

(event `self.ReceiveBeginPlay`
  ; Energy Logic
  (`self.UpdateBattery`))

(event `self.Drain`
  (params (Amount :type "Float (double-precision)"))
  ; Energy Logic
  (`/Game/IHaveADream/Core/Energy/AC_EnergyBase.DrainEnergy` (`self.AC_EnergyBase`) Amount)
  (`self.UpdateBattery`))

(event `self.Charge`
  (params (Amount :type "Float (double-precision)"))
  ; Energy Logic
  (`/Game/IHaveADream/Core/Energy/AC_EnergyBase.ChargeEnergy` (`self.AC_EnergyBase`) Amount)
  (`self.UpdateBattery`))

(event `UpdateBattery`
  (bind _output_get (set `self.LightLevel` (* (`/Game/IHaveADream/Core/Energy/AC_EnergyBase.EnergyProcentage` (`self.AC_EnergyBase`)) (`self.MaxLight`))))
  (`LightComponent.SetIntensity` (`self.PointLight`) _output_get))

(event `self.Box.OnComponentBeginOverlap`
  (params (OverlappedComponent :type "PrimitiveComponent Object Reference") (OtherActor :type "Actor Object Reference") (OtherComp :type "PrimitiveComponent Object Reference") (OtherBodyIndex :type Integer) (bFromSweep :type Boolean) (SweepResult :type "HitResult Structure (by ref)"))
  ; In
  (for _array_element (`Actor.Tags` OtherActor)
    (switch `name` _array_element
      (:`Player`
        ;; Player
        (bind _output_get (set `self.Player` OtherActor))
        (set `self.HasPlayer` true)
        (`CableComponent.SetAttachEndTo` (`self.EnergyCableToPlayer`) _output_get "CableBatteryPoint" "None")
        (`SceneComponent.SetVisibility` (`self.EnergyCableToPlayer`) true false))
      (:`PuzzleTrigger`
        ;; PuzzleTrigger
        (bind _output_get_2 (set `self.Puzzle` OtherActor))
        (bind _newparam (message `/Game/IHaveADream/Core/Energy/BPI_HasEnergy.GetEnergyComponent` _output_get_2))
        (set `self.PuzzleEnergyComponent` _newparam)
        (set `self.HasPuzzleTrigger` true)
        (`CableComponent.SetAttachEndTo` (`self.EnergyCableToPuzzle`) _output_get_2 "CableAttachPoint" "None")
        (`SceneComponent.SetVisibility` (`self.EnergyCableToPuzzle`) true false)))))

(event `self.Box.OnComponentEndOverlap`
  (params (OverlappedComponent :type "PrimitiveComponent Object Reference") (OtherActor :type "Actor Object Reference") (OtherComp :type "PrimitiveComponent Object Reference") (OtherBodyIndex :type Integer))
  ; Out
  (for _array_element (`Actor.Tags` OtherActor)
    (switch `name` _array_element
      (:`Player`
        ;; Player
        (`SceneComponent.SetVisibility` (`self.EnergyCableToPlayer`) false false)
        (`CableComponent.SetAttachEndTo` (`self.EnergyCableToPlayer`) self "None" "None")
        (set `self.Player` null)
        (set `self.HasPlayer` false))
      (:`PuzzleTrigger`
        ;; PuzzleTrigger
        (`SceneComponent.SetVisibility` (`self.EnergyCableToPuzzle`) false false)
        (`CableComponent.SetAttachEndTo` (`self.EnergyCableToPuzzle`) self "None" "None")
        (set `self.Puzzle` null)
        (set `self.PuzzleEnergyComp` null)
        (set `self.HasPuzzleTrigger` false)))))

(fn `UserConstructionScript`)