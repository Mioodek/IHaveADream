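; Lockable door actor that opens and closes through a timeline, triggered automatically by player overlap with its box or through an interaction event.
; The timeline drives hinge rotation or slide movement, selected by OpenOnUnlock, which also makes the door open when unlocked.
; Destroying the referenced Key unlocks the door.
; Timeline completion checks play direction to set the open state and fire open or close callbacks.
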(event `OnDoorOpen`
  ;[0.15 0.01094 0.02766 0.5] Custom events
  (if (not (`self.IsLocked`))
    (bind _direction (`Timeline|DoorOpening` :!label _label)
      (:`Update`
        (`self.SetHingePosition` 0.0 (`self.OpenAngle`))
        (`self.SetSlidePosition` 0.0 (`self.SlideDistance`) (`self.SlideDirection`)))
      (:`Finished`
        ;; To check whether it was reversed or not
        (switch `ETimelineDirection` _direction
          (:`Forward`
            (set `self.IsDoorOpen` true)
            (`self.OnOpen`))
          (:`Backward`
            (set `self.IsDoorOpen` false)
            (`self.OnClose`)))))))

(event `OnDoorClose`
  ;[0.15 0.01094 0.02766 0.5] Custom events
  (if (not (`self.RemainOpen`))
    (goto _label :!via `Reverse`)))

(event `self.Box.OnComponentBeginOverlap`
  (params (OverlappedComponent :type "PrimitiveComponent Object Reference") (OtherActor :type "Actor Object Reference") (OtherComp :type "PrimitiveComponent Object Reference") (OtherBodyIndex :type Integer) (bFromSweep :type Boolean) (SweepResult :type "HitResult Structure (by ref)"))
  ;[0.02182 0.000571 0.15 0.5] Box Overlap Interaction
  (if (== OtherActor (`GameplayStatics.GetPlayerCharacter` 0))
    (if (`self.IsAutomaticOpen`)
      (`self.OnDoorOpen`)
      (else
        (`self.EnableInput` (`GameplayStatics.GetPlayerController` 0))))))

(event `self.Key.OnDestroyed`
  (params (DestroyedActor :type "Actor Object Reference"))
  ;[0 1 0.8094 0.5] Key unlock trigger
  (`self.UnlockDoor`))

(event `self.Box.OnComponentEndOverlap`
  (params (OverlappedComponent :type "PrimitiveComponent Object Reference") (OtherActor :type "Actor Object Reference") (OtherComp :type "PrimitiveComponent Object Reference") (OtherBodyIndex :type Integer))
  ;[0.02182 0.000571 0.15 0.5] Box Overlap Interaction
  (if (== OtherActor (`GameplayStatics.GetPlayerCharacter` 0))
    (if (`self.IsAutomaticClosed`)
      (`self.OnDoorClose`)
      (else
        (`self.DisableInput` (`GameplayStatics.GetPlayerController` 0))))))

(event `CustomEvent`
  (params (InteractingPlayer :type "Actor Object Reference"))
  ;[0.15 0.08827 0.02245 0.5] Input
  (if (== InteractingPlayer (`GameplayStatics.GetPlayerCharacter` 0))
    (if (`self.IsDoorOpen`)
      (`self.OnDoorClose`)
      (else
        (`self.OnDoorOpen`)))
    (else
      (`self.OnDoorOpen`))))

(fn `LockDoor`
  (set `self.IsLocked` true))

(fn `SetHingePosition`
  (params (Alpha :type "Float (double-precision)") (MaxHingeDistance :type "Float (double-precision)" :default 90.0))
  (if (not (`self.OpenOnUnlock`))
    (`SceneComponent.K2_SetRelativeRotation` (`self.Scene`) (`KismetMathLibrary.MakeRotator` 0.0 0.0 (`KismetMathLibrary.Lerp` 0.0 MaxHingeDistance Alpha)) false false)))

(fn `SetSlidePosition`
  (params (Alpha :type "Float (double-precision)") (MaxDistance :type "Float (double-precision)") (Direction :type "Vector Structure" :default (0.0 1.0 0.0)))
  (if (`self.OpenOnUnlock`)
    ;[0.15 0.129 0 0.5] O ile ma się przesunąć wybrać w wektorze funkcji
    (`SceneComponent.K2_SetRelativeLocation` (`self.Scene`) (* (`KismetMathLibrary.Normal` Direction) (`KismetMathLibrary.Lerp` 0.0 MaxDistance Alpha)) false false)))

(fn `UnlockDoor`
  (set `self.IsLocked` false)
  (`self.OnUnlock`)
  (if (`self.OpenOnUnlock`)
    (`self.OnDoorOpen`)))

(fn `UserConstructionScript`)