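; Electricity trap for environment puzzles that drains energy from overlapping actors that implement BPI_HasEnergy.
; A looping timer flip-flops the Niagara effect's visibility and a SupposedToDealDamage flag on a LifeTIme interval.
; Box overlaps maintain the ToDrain list, running a tenth-second timer while it has occupants to apply Dps as drain.
; DamageOverTime never checks SupposedToDealDamage, so the drain logic ignores the hidden phase.
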(event `LifespanStarter`
  (`KismetSystemLibrary.K2_SetTimerDelegate` (delegate `HidingLogic`) (`self.LifeTIme`) true))

(event `HidingLogic`
  (bind _niagara (`self.Niagara`))
  (`/Engine/EditorBlueprintResources/StandardMacros.FlipFlop`
    (:`A`
      (`SceneComponent.SetHiddenInGame` _niagara true false)
      (set `self.SupposedToDealDamage?` false)
      (`KismetSystemLibrary.PrintString` "Hello"))
    (:`B`
      (`SceneComponent.SetHiddenInGame` _niagara false false)
      (set `self.SupposedToDealDamage?` true))))

(event `self.ReceiveBeginPlay`
  (bind _returnvalue (`KismetSystemLibrary.K2_SetTimerDelegate` (`|CreateDelegate` :!event `DamageOverTime`) 0.1 true))
  (bind _output_get (set `self.TimerByEvent` _returnvalue))
  (`KismetSystemLibrary.K2_PauseTimerHandle` _output_get)
  (`self.LifespanStarter`))

(event `self.Box.OnComponentBeginOverlap`
  (params (OverlappedComponent :type "PrimitiveComponent Object Reference") (OtherActor :type "Actor Object Reference") (OtherComp :type "PrimitiveComponent Object Reference") (OtherBodyIndex :type Integer) (bFromSweep :type Boolean) (SweepResult :type "HitResult Structure (by ref)"))
  (if (`KismetSystemLibrary.DoesImplementInterface` OtherActor "/Game/IHaveADream/Core/Energy/BPI_HasEnergy.BPI_HasEnergy_C")
    (bind _asbpi_has_energy (cast `/Game/IHaveADream/Core/Energy/BPI_HasEnergy` OtherActor))
    (`KismetArrayLibrary.Array_AddUnique` (`self.ToDrain`) _asbpi_has_energy)
    (`KismetSystemLibrary.K2_UnPauseTimerHandle` (`self.TimerByEvent`))))

(event `self.Box.OnComponentEndOverlap`
  (params (OverlappedComponent :type "PrimitiveComponent Object Reference") (OtherActor :type "Actor Object Reference") (OtherComp :type "PrimitiveComponent Object Reference") (OtherBodyIndex :type Integer))
  (if (`KismetSystemLibrary.DoesImplementInterface` OtherActor "/Game/IHaveADream/Core/Energy/BPI_HasEnergy.BPI_HasEnergy_C")
    (bind _asbpi_has_energy (cast `/Game/IHaveADream/Core/Energy/BPI_HasEnergy` OtherActor))
    (`KismetArrayLibrary.Array_RemoveItem` (`self.ToDrain`) _asbpi_has_energy)
    (if (`KismetArrayLibrary.Array_IsEmpty` (`self.ToDrain`))
      (`KismetSystemLibrary.K2_PauseTimerHandle` (`self.TimerByEvent`)))))

(event `DamageOverTime`
  (`/Game/IHaveADream/Core/Energy/BPI_HasEnergy.DrainEnergy` (`self.ToDrain`) (/ (`self.dps`) 10.0)))

(fn `UserConstructionScript`)