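; BP_ToxicWater is a toxic water trap with a box trigger meant to deal periodic damage.
; A BP_FirstPersonCharacter entering the box starts a looping half-second timer that calls DealDamage.
; DealDamage loops over every overlapping actor but only prints half of DamagePerSec, applying no actual damage.
; End overlap clears the timer when a class check passes and no actors remain in the box.
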(event `self.Box.OnComponentEndOverlap`
  (params (OverlappedComponent :type "PrimitiveComponent Object Reference") (OtherActor :type "Actor Object Reference") (OtherComp :type "PrimitiveComponent Object Reference") (OtherBodyIndex :type Integer))
  (`KismetSystemLibrary.IsObjectOfSoftClass` OtherActor
    (:`True`
      (if (`KismetArrayLibrary.Array_IsEmpty` (`PrimitiveComponent.GetOverlappingActors` (`self.Box`) "/Script/Engine.Actor"))
        (`KismetSystemLibrary.K2_ClearAndInvalidateTimerHandle` (stale `self.Box.OnComponentBeginOverlap` _output_get))))))

(event `self.Box.OnComponentBeginOverlap`
  (params (OverlappedComponent :type "PrimitiveComponent Object Reference") (OtherActor :type "Actor Object Reference") (OtherComp :type "PrimitiveComponent Object Reference") (OtherBodyIndex :type Integer) (bFromSweep :type Boolean) (SweepResult :type "HitResult Structure (by ref)"))
  (`KismetSystemLibrary.IsObjectOfSoftClass` OtherActor "/Game/IHaveADream/Player/BP_FirstPersonCharacter.BP_FirstPersonCharacter_C"
    (:`True`
      (bind _returnvalue (`KismetSystemLibrary.K2_SetTimerDelegate` (delegate `DealDamage`) 0.5 true))
      (bind _output_get (set `self.TimerHandle Area of Damage` _returnvalue)))))

(event `DealDamage`
  (for _ (`PrimitiveComponent.GetOverlappingActors` (`self.Box`) "/Script/Engine.Actor")
    (`KismetSystemLibrary.PrintString` (`KismetStringLibrary.Conv_DoubleToString` (/ (`self.DamagePerSec`) 2.0)))))

(fn `UserConstructionScript`)