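; Closing-wall trap that slows the player and moves a wall, with crush detection that only prints a death placeholder.
; After a short delay, trigger overlap drops walk speed to a crawl and plays a timeline lerping the wall toward its scaled forward vector as a world position.
; Leaving the trigger restores speed.
; Two boxes share one boolean, so a second player overlap while it is set prints the placeholder.
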(event `self.Trigger.OnComponentBeginOverlap`
  (params (OverlappedComponent :type "PrimitiveComponent Object Reference") (OtherActor :type "Actor Object Reference") (OtherComp :type "PrimitiveComponent Object Reference") (OtherBodyIndex :type Integer) (bFromSweep :type Boolean) (SweepResult :type "HitResult Structure (by ref)"))
  (bind _movingwall (`self.MovingWall`))
  ; ClosingWallTrigger
  (`KismetSystemLibrary.Delay` 0.5)
  (bind _asbp_first_person_character (cast `/Game/IHaveADream/Player/BP_FirstPersonCharacter` OtherActor))
  (bind _charactermovement (`Character.CharacterMovement` _asbp_first_person_character))
  (set `self.PlayerDefaultMovementSpeed` (`CharacterMovementComponent.MaxWalkSpeed` _charactermovement))
  (set `CharacterMovementComponent.MaxWalkSpeed` 1.0 _charactermovement)
  (bind (_direction _newtrack_0) (`Timeline|Timeline`)
    (:`Update`
      (`SceneComponent.K2_SetWorldLocation` (`self.MovingWall`) (`KismetMathLibrary.VLerp` (`SceneComponent.K2_GetComponentLocation` _movingwall) (* (`SceneComponent.GetForwardVector` _movingwall) 50.0) (* _newtrack_0 (`self.Speed`))) false false))))

(event `self.Trigger.OnComponentEndOverlap`
  (params (OverlappedComponent :type "PrimitiveComponent Object Reference") (OtherActor :type "Actor Object Reference") (OtherComp :type "PrimitiveComponent Object Reference") (OtherBodyIndex :type Integer))
  ; Returning Default Player's Movement Speed
  (bind _asbp_first_person_character (cast `/Game/IHaveADream/Player/BP_FirstPersonCharacter` OtherActor))
  (set `CharacterMovementComponent.MaxWalkSpeed` (`self.PlayerDefaultMovementSpeed`) (`Character.CharacterMovement` _asbp_first_person_character)))

(event `self.Box1.OnComponentBeginOverlap`
  (params (OverlappedComponent :type "PrimitiveComponent Object Reference") (OtherActor :type "Actor Object Reference") (OtherComp :type "PrimitiveComponent Object Reference") (OtherBodyIndex :type Integer) (bFromSweep :type Boolean) (SweepResult :type "HitResult Structure (by ref)"))
  (cast `/Game/IHaveADream/Player/BP_FirstPersonCharacter` OtherActor)
  (if (`self.IsCollidingWithWall`)
    (`KismetSystemLibrary.PrintString` "PLACE DEATH EVENT HERE")
    (else
      (set `self.IsCollidingWithWall` true))))

(event `self.Box2.OnComponentBeginOverlap`
  (params (OverlappedComponent :type "PrimitiveComponent Object Reference") (OtherActor :type "Actor Object Reference") (OtherComp :type "PrimitiveComponent Object Reference") (OtherBodyIndex :type Integer) (bFromSweep :type Boolean) (SweepResult :type "HitResult Structure (by ref)"))
  (cast `/Game/IHaveADream/Player/BP_FirstPersonCharacter` OtherActor)
  (if (`self.IsCollidingWithWall`)
    (`KismetSystemLibrary.PrintString` "PLACE DEATH EVENT HERE")
    (else
      (set `self.IsCollidingWithWall` true))))

(event `self.Box2.OnComponentEndOverlap`
  (params (OverlappedComponent :type "PrimitiveComponent Object Reference") (OtherActor :type "Actor Object Reference") (OtherComp :type "PrimitiveComponent Object Reference") (OtherBodyIndex :type Integer))
  ; Boolean Return to false
  (`KismetSystemLibrary.IsObjectOfSoftClass` OtherActor "/Game/IHaveADream/Player/BP_FirstPersonCharacter.BP_FirstPersonCharacter_C"
    (:`True`
      (set `self.IsCollidingWithWall` false :!label _label))))

(event `self.Box1.OnComponentEndOverlap`
  (params (OverlappedComponent :type "PrimitiveComponent Object Reference") (OtherActor :type "Actor Object Reference") (OtherComp :type "PrimitiveComponent Object Reference") (OtherBodyIndex :type Integer))
  ; Boolean Return to false
  (`KismetSystemLibrary.IsObjectOfSoftClass` OtherActor "/Game/IHaveADream/Player/BP_FirstPersonCharacter.BP_FirstPersonCharacter_C"
    (:`True`
      (goto _label))))

(fn `UserConstructionScript`)