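; BP_Turret is a trap turret that sweeps back and forth, then fires on sighted pawns tagged TurretTarget.
; Tick switches between searching, which rotates the poseable mesh within a yaw arc, and attacking.
; PawnSensing stores the target location, snaps the mesh toward it and restarts a one-second timer back to searching.
; Attacks spawn BP_TurretProjectile aimed at that location, using delays and a shot counter to fire in bursts.
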(event `self.ReceiveTick`
  (params (DeltaSeconds :type "Float (single-precision)"))
  ; State Switcher
  (switch `/Game/IHaveADream/Gameplay/Traps/Turret/ENUM_TurretState` (`self.TurretState`)
    (:`NewEnumerator0`
      (`self.Rotate Turret`))
    (:`NewEnumerator1`
      (`self.TurretAttack`))))

(event `Rotate Turret`
  (bind _returnvalue (* (`GameplayStatics.GetWorldDeltaSeconds`) 50.0))
  (bind _relativerotation (`SceneComponent.RelativeRotation` (`self.PoseableMesh1`)))
  (bind _yaw (.yaw _relativerotation))
  (bind _yaw_2 (.yaw _relativerotation))
  (set `self.ShouldTurretRotateRight` (or (and (< _yaw_2 -20.0) (`self.ShouldTurretRotateRight`)) (and (< _yaw_2 -160.0) (not (`self.ShouldTurretRotateRight`)))))
  (`SceneComponent.K2_SetRelativeRotation` (`self.PoseableMesh1`) (`KismetMathLibrary.MakeRotator` (.roll _relativerotation) (.pitch _relativerotation) (`KismetMathLibrary.SelectFloat` (+ _yaw _returnvalue) (- _yaw _returnvalue) (`self.ShouldTurretRotateRight`))) false false))

(event `self.PawnSensing.OnSeePawn`
  (params (Pawn :type "Pawn Object Reference"))
  (bind _poseablemesh1 (`self.PoseableMesh1`))
  (bind (_returnvalue_roll _returnvalue_pitch _returnvalue_yaw) (`KismetMathLibrary.BreakRotator` (`KismetMathLibrary.FindLookAtRotation` (`self.K2_GetActorLocation`) (`self.TargetLocation`))))
  (bind (_returnvalue_roll_2 _returnvalue_pitch_2) (`KismetMathLibrary.BreakRotator` (`SceneComponent.K2_GetComponentRotation` _poseablemesh1)))
  (if (`self.ActorHasTag` Pawn "TurretTarget")
    (set `self.TargetLocation` (`self.K2_GetActorLocation` Pawn))
    (set `self.TurretState` "NewEnumerator1")
    (`SceneComponent.K2_SetWorldRotation` _poseablemesh1 (`KismetMathLibrary.MakeRotator` _returnvalue_roll_2 _returnvalue_pitch_2 (- _returnvalue_yaw 90.0)) false false)
    (`KismetSystemLibrary.K2_ClearAndInvalidateTimerHandle` (`self.ResetTurretState`))
    (bind _returnvalue (`KismetSystemLibrary.K2_SetTimerDelegate` (delegate `Reset Turret State`) 1.0))
    (set `self.ResetTurretState` _returnvalue)))

(event `Reset Turret State`
  (set `self.TurretState` "NewEnumerator0"))

(event `TurretAttack`
  (bind _returnvalue (`SceneComponent.K2_GetComponentLocation` (`self.Arrow`)))
  (bind _returnvalue_2 (`KismetMathLibrary.GetDirectionUnitVector` _returnvalue (`self.TargetLocation`)))
  ; AttackLogic
  (if (not (`self.IsAttacking?`))
    (set `self.IsAttacking?` true)
    (bind _returnvalue_3 (`|SpawnActorFromClass` "/Game/IHaveADream/Gameplay/Traps/Turret/BP_TurretProjectile.BP_TurretProjectile_C" (`KismetMathLibrary.MakeTransform` (+ _returnvalue (* _returnvalue_2 60.0))) "Undefined" "MultiplyWithRoot" null null))
    (set `MovementComponent.Velocity` (* _returnvalue_2 3000.0) (`/Game/IHaveADream/Gameplay/Traps/Turret/BP_TurretProjectile.ProjectileMovement` _returnvalue_3))
    (`KismetSystemLibrary.Delay` (`self.DelayBetweenAttacks`))
    (bind _result (`/Engine/EditorBlueprintResources/StandardMacros.IncrementInt` (`self.NumberOfAttacksDone`))
      (:`  `
        (if (>= _result (`self.AttackFrequency`))
          (set `self.NumberOfAttacksDone` 0)
          (`KismetSystemLibrary.Delay` (`self.DelayBetweenMultipleAttacks`)))
        (set `self.IsAttacking?` false)))))

(fn `UserConstructionScript`)