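; Panel actor that opens the W_Labirynth minigame widget when a player-tagged actor overlaps its trigger.
; On overlap it passes itself to the new widget, switches input to UI only and shows the mouse cursor.
; Succes and Fail events print debug text and fire the same PanelActorTest dispatcher, bound on BeginPlay.
; Its handler removes the widget and restores game-only input, so both outcomes currently end identically.
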(event `self.Trigger.OnComponentBeginOverlap`
  (params (OverlappedComponent :type "PrimitiveComponent Object Reference") (OtherActor :type "Actor Object Reference") (OtherComp :type "PrimitiveComponent Object Reference") (OtherBodyIndex :type Integer) (bFromSweep :type Boolean) (SweepResult :type "HitResult Structure (by ref)"))
  (bind _returnvalue (`GameplayStatics.GetPlayerController` 0))
  (if (`self.ActorHasTag` OtherActor "Player")
    (bind _returnvalue_2 (`|CreateWidget` "/Game/LemGame/MiniGames/MiniGameWidget/Labirynt/W_Labirynth.W_Labirynth_C" null self))
    (set `self.WidgetMiniGame` _returnvalue_2)
    (`UserWidget.AddToPlayerScreen` _returnvalue_2 0)
    (`WidgetBlueprintLibrary.SetInputMode_UIOnlyEx` _returnvalue _returnvalue_2)
    (set `PlayerController.bShowMouseCursor` true _returnvalue)))

(event `self.ReceiveBeginPlay`
  (add `self.PanelActorTest` (delegate `PanelActorTest_Event`)))

(event `PanelActorTest_Event`
  (bind _returnvalue (`GameplayStatics.GetPlayerController` 0))
  (bind _widgetminigame (`self.WidgetMiniGame`))
  (`Widget.SetVisibility` _widgetminigame "Hidden")
  (`Widget.RemoveFromParent` _widgetminigame)
  (`WidgetBlueprintLibrary.SetInputMode_GameOnly` _returnvalue)
  (set `PlayerController.bShowMouseCursor` false _returnvalue))

(event `Succes`
  (`KismetSystemLibrary.PrintString` "succes in actor")
  (`self.PanelActorTest_Event`))

(event `Fail`
  (`KismetSystemLibrary.PrintString` "fail in actor")
  (`self.PanelActorTest_Event`))

(fn `UserConstructionScript`)